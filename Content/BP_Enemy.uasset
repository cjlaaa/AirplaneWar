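; BP_Enemy is an enemy ship actor that randomizes its colors and scales in when its SetColor event runs.
; SetColor picks random body and wing color indices, each from its own four-color palette.
; It creates dynamic material instances from BasicShapeMaterial for the hull mesh and for both wing meshes, which share one.
; It then plays SpawnScaleTimeline to drive the actor's uniform scale.
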(event EventBeginPlay)

(event Collision|EventActorBeginOverlap
  (params (OtherActor :type Actor%20Object%20Reference)))

(event EventTick
  (params (DeltaSeconds :type Float%20%28single-precision%29)))

(event EventSetColor
  (Variables|Default|SetBodyColorIndex (Math|Random|RandomIntegerinRange 0 3))
  (Variables|Default|SetWingColorIndex (Math|Random|RandomIntegerinRange 0 3))
  (bind _returnvalue (Rendering|Material|CreateDynamicMaterialInstance "/Engine/BasicShapes/BasicShapeMaterial.BasicShapeMaterial" "None" :!class /Script/Engine.KismetMaterialLibrary))
  (Rendering|Material|SetVectorParameterValue _returnvalue "Color" (Utilities|Select :Index (Variables|Default|GetBodyColorIndex) :Option%200 "(R=1.000000,G=0.000000,B=0.000000,A=1.000000)" :Option%201 "(R=0.420606,G=0.000000,B=1.000000,A=1.000000)" :Option%202 "(R=0.000000,G=1.000000,B=0.044180,A=1.000000)" :Option%203 "(R=1.000000,G=0.996939,B=0.000000,A=1.000000)") :!class /Script/Engine.MaterialInstanceDynamic)
  (Rendering|Material|SetMaterial (Variables|Default|GetShipSM) 0 _returnvalue)
  (bind _returnvalue_2 (Rendering|Material|CreateDynamicMaterialInstance "/Engine/BasicShapes/BasicShapeMaterial.BasicShapeMaterial" "None" :!class /Script/Engine.KismetMaterialLibrary))
  (Rendering|Material|SetVectorParameterValue _returnvalue_2 "Color" (Utilities|Select :Index (Variables|Default|GetWingColorIndex) :Option%200 "(R=1.000000,G=0.000000,B=0.883618,A=1.000000)" :Option%201 "(R=0.000000,G=0.919867,B=1.000000,A=1.000000)" :Option%202 "(R=1.000000,G=0.496533,B=0.000000,A=1.000000)" :Option%203 "(R=0.000000,G=0.074900,B=0.870000,A=1.000000)") :!class /Script/Engine.MaterialInstanceDynamic)
  (Rendering|Material|SetMaterial (Variables|Default|GetWingSM2) 0 _returnvalue_2)
  (Rendering|Material|SetMaterial (Variables|Default|GetWingSM1) 0 _returnvalue_2)
  (bind _scale (Timeline|SpawnScaleTimeline Play)
    (:Update
      (Transformation|SetActorScale3D (Math|Conversions|ToVector(Float) _scale)))))

(fn ConstructionScript)